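; BP_TankPawn is a tank pawn that links player input to interaction, save UI and quest list visibility.
; Input actions call the InteractionComponent, add one of two save widgets to the viewport, or toggle the quest list.
; BeginPlay records whether player controller 0 possesses the tank; if so, EndPlay shows the main menu through BP_MenuHud.
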(event Collision|EventActorBeginOverlap
  (params (OtherActor :type Actor%20Object%20Reference)))

(event EventTick
  (params (DeltaSeconds :type Float%20%28single-precision%29)))

(event EventEndPlay
  (params (EndPlayReason :type EEndPlayReason%20Enum :default "Destroyed"))
  (if (stale EventBeginPlay _output_get)
    (bind _asbp_menu_hud (Utilities|Casting|CastToBP_MenuHud (HUD|GetHUD (Game|GetPlayerController 0))))
    (Class|MenuHud|ShowWindow _asbp_menu_hud "MainMenu")))

(event EventBeginPlay
  (bind _output_get (Variables|Default|SetCrtl (== (Pawn|GetController) (Game|GetPlayerController 0)))))

(event Input|ActionEvents|InputActionInteraction
  (params (Key :type Key%20Structure :default "None"))
  (:Pressed
    (Class|InteractionComponent|Interact (Variables|Default|GetInteractionComponent))))

(event Input|ActionEvents|InputActionSave
  (params (Key :type Key%20Structure :default "None"))
  (:Pressed
    (bind _returnvalue (UserInterface|CreateWidget "/Game/Widgets/W_Saving.W_Saving_C" (Game|GetPlayerController 0)))
    (UserInterface|Viewport|AddtoViewport _returnvalue 0)))

(event Input|ActionEvents|InputActionSave2.0
  (params (Key :type Key%20Structure :default "None"))
  (:Pressed
    (bind _returnvalue (UserInterface|CreateWidget "/Game/Widgets/WBP_SaveLoadMenu.WBP_SaveLoadMenu_C" (Game|GetPlayerController 0)))
    (UserInterface|Viewport|AddtoViewport _returnvalue 0)))

(event Input|ActionEvents|InputActionToogle
  (params (Key :type Key%20Structure :default "None"))
  (:Pressed
    (Class|TankPawn|ToggleQuestListVisibility)))

(fn ConstructionScript)